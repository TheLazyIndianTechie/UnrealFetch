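; Test actor that fetches an account balance from a custom Hedera REST API when play begins.
; BeginPlay sends a Fetch request to a hardcoded URL with an API key header, binding an OnJson callback.
; The callback prints the nested data balance and the raw response text on screen.
; A separate debug graph holds a plain-text response printer that is never bound.
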(event `self.ReceiveBeginPlay`
  (bind _returnvalue (`FetchAPI.Fetch` "https://custom-hedera-rest-api.vercel.app/api/account/balance" (make `FetchOptions` "GET" "" (`|MakeArray` (make `FetchHeader` "x-api-key" "thelazyindiantechie")))))
  (`FetchRequest.OnJson` _returnvalue (delegate `CustomEvent-OnJSON`)))

(event `CustomOnTextEvent`
  (params (TextContent :type String) (Response :type "FetchResponse Object Reference"))
  (`KismetSystemLibrary.PrintString` TextContent true true (struct :`G` 0.66 :`B` 1.0 :`A` 1.0) 60.0))

(event `CustomEvent-OnJSON`
  (params (JsonValue :type "SimpleJsonValue Object Reference") (Response :type "FetchResponse Object Reference"))
  (`KismetSystemLibrary.PrintString` (`SimpleJsonObject.GetString` (`SimpleJsonObject.GetObject` (`SimpleJsonValue.AsObject` JsonValue) "data") "balance") true true (struct :`G` 0.66 :`B` 1.0 :`A` 1.0) 60.0)
  (`KismetSystemLibrary.PrintString` (`FetchResponse.ResponseText` Response) true true (struct :`G` 0.66 :`B` 1.0 :`A` 1.0) 120.0))

(fn `UserConstructionScript`)